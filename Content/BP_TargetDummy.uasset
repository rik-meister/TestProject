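; BP_TargetDummy is a test target actor that reports which side of its TargetCube was struck.
; On each component hit, it dots the negated, normalized hit normal with the cube's forward vector.
; Thresholds on that dot product classify the hit as front, back or side, and the result is only printed as a debug string.
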(event `self.TargetCube.OnComponentHit`
  (params (HitComponent :type "PrimitiveComponent Object Reference") (OtherActor :type "Actor Object Reference") (OtherComp :type "PrimitiveComponent Object Reference") (NormalImpulse :type "Vector Structure") (Hit :type "HitResult Structure (by ref)"))
  (bind _returnvalue (`KismetMathLibrary.Dot_VectorVector` (`KismetMathLibrary.Normal` (* (`.Normal` (`GameplayStatics.BreakHitResult` Hit)) -1.0)) (`SceneComponent.GetForwardVector` (`self.TargetCube`))))
  (if (> _returnvalue 0.5)
    (`KismetSystemLibrary.PrintString` "Front Hit")
    (elif (< _returnvalue -0.5)
      (`KismetSystemLibrary.PrintString` "Back Hit")
      (else
        (`KismetSystemLibrary.PrintString` "Side Hit")))))

(fn `UserConstructionScript`)