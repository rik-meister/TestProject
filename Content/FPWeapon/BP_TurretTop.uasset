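; BP_TurretTop is a turret head that tracks the player pawn and fires chicken projectiles at it.
; Each tick, while the player is within DetectionRange, a dot product checks alignment and a cross product's Z sign picks the yaw direction to turn at RotationSpeed.
; Once nearly aligned, it stops turning and spawns an impulse-launched BP_ChickenProjectile at BulletSpawner every tick, with no cooldown.
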(event `self.ReceiveBeginPlay`
  ;[1 1 1] Turret Action
  ;;[0 0.5997 1] Getting and reading player location
  (set `self.PlayerRef` (`GameplayStatics.GetPlayerPawn` 0)))

(event `self.ReceiveTick`
  (params (DeltaSeconds :type "Float (single-precision)"))
  (bind _returnvalue (`self.GetActorForwardVector`))
  (bind _bullet_spawner (`self.Bullet Spawner`))
  (bind _playerref (`self.PlayerRef`))
  (bind _returnvalue_2 (- (`self.K2_GetActorLocation` _playerref) (`self.K2_GetActorLocation`)))
  (bind _returnvalue_3 (`KismetMathLibrary.Normal` _returnvalue_2))
  (bind (_returnvalue_x _returnvalue_y _returnvalue_z) (`KismetMathLibrary.BreakVector` (`KismetMathLibrary.Cross_VectorVector` _returnvalue_3 _returnvalue)))
  ;[1 1 1] Turret Action
  ;;[0 0.5997 1] Getting and reading player location
  (if (`KismetSystemLibrary.IsValid` _playerref)
    (`/Engine/EditorBlueprintResources/StandardMacros.CompareFloat` (`KismetMathLibrary.VSize` _returnvalue_2) (`self.DetectionRange`)
      (:`<`
        (if true
          (if (> (`KismetMathLibrary.Dot_VectorVector` _returnvalue _returnvalue_3) 0.99)
            ;;[1 0 0] Shooting
            (bind _returnvalue_4 (`|SpawnActorFromClass` "/Game/BP_ChickenProjectile.BP_ChickenProjectile_C" (`SceneComponent.K2_GetComponentToWorld` _bullet_spawner) "Undefined" "MultiplyWithRoot" null null))
            (`PrimitiveComponent.AddImpulse` (`/Game/BP_ChickenProjectile.projectile` _returnvalue_4) (* (`SceneComponent.GetForwardVector` _bullet_spawner) 40000.0) "None" false)
            (else
              ;;[1 0.8289 0.06221] Moves Turret if it's not facing the player
              (if (> (* _returnvalue_z -1.0) 0.0)
                (`self.K2_AddActorLocalRotation` (`KismetMathLibrary.MakeRotator` 0.0 0.0 (* (`GameplayStatics.GetWorldDeltaSeconds`) (`self.RotationSpeed`))))
                (else
                  (`self.K2_AddActorLocalRotation` (`KismetMathLibrary.MakeRotator` 0.0 0.0 (* (`GameplayStatics.GetWorldDeltaSeconds`) (`self.RotationSpeed`) -1.0))))))))))))

(fn `UserConstructionScript`)